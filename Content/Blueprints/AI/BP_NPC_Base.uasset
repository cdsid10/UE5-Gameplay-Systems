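; Base NPC actor that players can interact with to open a dialogue from its NPC data.
; Interact caches the first interactor as the player, opens dialogue, then sets the interacting flag locally and in the BB_NPC blackboard through the AI controller.
; While that flag is set, Tick smoothly rotates the NPC toward the player.
; EndInteraction only closes the interactor's dialogue, leaving the flag unchanged.
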(event EventEndInteraction
  (params (Interactor :type BP%20Third%20Person%20Character%20Object%20Reference))
  (Default|CloseDialogue Interactor))

(event EventInteract
  (params (Interactor :type BP%20Third%20Person%20Character%20Object%20Reference))
  (Utilities|IsValid (Variables|Default|GetPlayerCharacter)
    (:Is%20Valid
      _)
    (:Is%20Not%20Valid
      (Variables|Default|SetPlayerCharacter Interactor)))
  (Default|OpenDialogue (Variables|Default|GetPlayerCharacter) (Variables|NPC_Data|GetNPC_Data))
  (CallFunction|SetIsInteractinginBB (Pawn|GetController) true))

(event EventTick
  (params (DeltaSeconds :type Float%20%28single-precision%29))
  (if (Variables|Default|GetIsInteracting)
    (Transformation|SetActorRotation (Math|Interpolation|RInterpTo (Transformation|GetActorRotation) (Math|Rotator|FindLookatRotation (Transformation|GetActorLocation) (Transformation|GetActorLocation (Variables|Default|GetPlayerCharacter))) (Utilities|Time|GetWorldDeltaSeconds) 5.0))))

(fn ConstructionScript)

(fn SetIsInteractinginBB
  (params (AI%20Controller :type Object%20Object%20Reference) (IsInteracting :type Boolean))
  (bind _asbp_ai_controller (Utilities|Casting|CastToBP_AI_Controller AI%20Controller))
  (bind _blackboardcomponent (Class|AIController|UseBlackboard _asbp_ai_controller "/Game/Blueprints/AI/BT/BB_NPC.BB_NPC"))
  (AI|Components|Blackboard|SetValueasBool _blackboardcomponent (Variables|Default|GetIsInteractingBBName) IsInteracting)
  (Variables|Default|SetIsInteracting IsInteracting))