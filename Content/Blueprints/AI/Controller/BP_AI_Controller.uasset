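; BP_AI_Controller is the AI controller for NPCs that walk a looping patrol route.
; On BeginPlay it runs BT_NPC with BB_NPC and copies the patrol points from the possessed BP_NPC_Base.
; It writes the current point to the PatrolTarget blackboard key.
; Each successful move-completed event advances the index, wraps it to the start, and updates that key.
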(event Custom|OnMoveCompleted
  (params (RequestID :type AI%20Request%20ID%20Structure) (Result :type EPathFollowingResult%20Enum :default "Success"))
  (if (Utilities|Enum|Equal(Enum) Result "Success")
    (bind _result (Math|Integer|IncrementInt (Variables|Default|GetCurrentPatrolIndex))
      (:%20%20
        (Variables|Default|SetCurrentPatrolIndex _result)
        (if (>= (Variables|Default|GetCurrentPatrolIndex) (Utilities|Array|Length (Variables|Default|GetPatrolPoints)))
          (Variables|Default|SetCurrentPatrolIndex 0))
        (AI|Components|Blackboard|SetValueasObject (Variables|Default|GetBlackboard) (Variables|Default|GetPatrolTarget) (Utilities|Array|Get(acopy) (Variables|Default|GetPatrolPoints) (Variables|Default|GetCurrentPatrolIndex)))))))

(event EventBeginPlay
  (AI|RunBehaviorTree "/Game/Blueprints/AI/BT/BT_NPC.BT_NPC")
  (EventDispatchers|BindEventtoReceiveMoveCompleted (delegate Custom|OnMoveCompleted))
  (Class|AIController|UseBlackboard "/Game/Blueprints/AI/BT/BB_NPC.BB_NPC")
  (bind _asbp_npc_base (Utilities|Casting|CastToBP_NPC_Base (Pawn|GetControlledPawn)))
  (Variables|Default|SetPatrolPoints (Variables|/Game/Blueprints/AI/BP_NPC_Base.BP_NPC_Base_C|GetPatrolPoints _asbp_npc_base))
  (AI|Components|Blackboard|SetValueasObject (Variables|Default|GetBlackboard) (Variables|Default|GetPatrolTarget) (Utilities|Array|Get(acopy) (Variables|Default|GetPatrolPoints) (Variables|Default|GetCurrentPatrolIndex))))

(fn ConstructionScript)