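; Inventory component that stores item ID and quantity stacks for its owner, starting with a phone battery.
; Adding merges into an existing stack or appends, with items looked up in DT_ItemDataTable.
; Dropping one unit or the last merges into a matching nearby pickup found by sphere overlap, otherwise spawns one ahead of the owner.
; A use function consumes quantity and reports success; changes call OnInventoryChanged.
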(event EventBeginPlay
  (CallFunction|AddItem (Utilities|Struct|MakeST_ItemData "PhoneBattery" 1)))

(event EventTick
  (params (DeltaSeconds :type Float%20%28single-precision%29)))

(fn AddItem
  (params (NewItem :type ST%20Item%20Data%20Structure))
  (bind _output_get (LocalVariables|SetNewItemData NewItem))
  (bind _returnvalue (Utilities|GetDataTableRow "/Game/Blueprints/Data/DT_ItemDataTable.DT_ItemDataTable" (.itemid _output_get))
    (:then
      (LocalVariables|SetNewItemDetails _returnvalue)
      (bind (_array_element _array_index) (Utilities|Array|ForEachLoopwithBreak (Variables|Default|GetInventoryItems) :!label _label)
        (:LoopBody
          (LocalVariables|SetCurrentArrayIndex _array_index)
          (bind _output_get_2 (LocalVariables|SetFoundItem (== (.ItemID (Utilities|Struct|BreakST_ItemData _array_element)) (.ItemID (Utilities|Struct|BreakST_ItemData (LocalVariables|GetNewItemData))))))
          (if _output_get_2
            (CallFunction|AddItemQuantitytoInventory (LocalVariables|GetCurrentArrayIndex) (LocalVariables|GetNewItemData))
            (Default|CallOnInventoryChanged)
            (goto _label Break)))
        (:Completed
          (if (not (LocalVariables|GetFoundItem))
            (Utilities|Array|Add (Variables|Default|GetInventoryItems) (LocalVariables|GetNewItemData))
            (Development|PrintString (Utilities|String|Append (Utilities|String|ToString(Name) (.itemname (LocalVariables|GetNewItemDetails))) " Has been picked up!" "With Quantity: " (Utilities|String|ToString(Integer) (.Quantity (Utilities|Struct|BreakST_ItemData (LocalVariables|GetNewItemData))))))
            (Default|CallOnInventoryChanged)))))))

(fn AddItemQuantitytoInventory
  (params (CurrentArrayIndex :type Integer) (NewItemData :type ST%20Item%20Data%20Structure))
  (bind (_itemid _quantity) (Utilities|Struct|BreakST_ItemData NewItemData))
  (LocalVariables|SetCurrentIndex CurrentArrayIndex)
  (Utilities|GetDataTableRow "/Game/Blueprints/Data/DT_ItemDataTable.DT_ItemDataTable" (.ItemID (Utilities|Struct|BreakST_ItemData NewItemData))
    (:then
      (Utilities|Array|SetArrayElem (Variables|Default|GetInventoryItems) (LocalVariables|GetCurrentIndex) (Utilities|Struct|MakeST_ItemData _itemid (+ (.Quantity (Utilities|Struct|BreakST_ItemData (Utilities|Array|Get(acopy) (Variables|Default|GetInventoryItems) (LocalVariables|GetCurrentIndex)))) _quantity))))))

(fn DropItemfromInventory
  (params (Index :type Integer))
  (LocalVariables|SetCurrentIndex Index)
  (if (> (.Quantity (Utilities|Struct|BreakST_ItemData (Utilities|Array|Get(acopy) (Variables|Default|GetInventoryItems) (LocalVariables|GetCurrentIndex)))) 1)
    (CallFunction|DropItemQuantityfromInventory (LocalVariables|GetCurrentIndex) (Utilities|Array|Get(acopy) (Variables|Default|GetInventoryItems) (LocalVariables|GetCurrentIndex)))
    (else
      (CallFunction|DropAllItemsfromInventory (LocalVariables|GetCurrentIndex))))
  (Default|CallOnInventoryChanged))

(fn DropItemQuantityfromInventory
  (params (CurrentArrayIndex :type Integer) (ArrayItem :type ST%20Item%20Data%20Structure))
  (bind _returnvalue (Components|GetOwner))
  (bind _inventoryitems (Variables|Default|GetInventoryItems))
  (bind _returnvalue_2 (Transformation|GetActorLocation _returnvalue))
  (bind _output (Utilities|Array|Get(acopy) _inventoryitems CurrentArrayIndex))
  (bind (_itemid _quantity) (Utilities|Struct|BreakST_ItemData _output))
  (bind _returnvalue_3 (Utilities|GetDataTableRow "/Game/Blueprints/Data/DT_ItemDataTable.DT_ItemDataTable" (.ItemID (Utilities|Struct|BreakST_ItemData ArrayItem)))
    (:then
      (bind _output_get (LocalVariables|SetNewItemDetails _returnvalue_3))
      (LocalVariables|SetItemClassToSpawn (.itempickupclass _output_get))
      ;[0.15 0.15 0.15 0.5] Check For Item Already in world, if yes then add to its quantity instead of spawning a new one
      (bind _outactors (Collision|SphereOverlapActors _returnvalue_2 128.0 (LocalVariables|GetObjectTypeQuery) "/Game/Blueprints/Items/BP_ItemPickup.BP_ItemPickup_C"))
      (bind _array_element (Utilities|Array|ForEachLoopwithBreak _outactors :!label _label)
        (:LoopBody
          (bind _asbp_item_pickup (Utilities|Casting|CastToBP_ItemPickup _array_element))
          (if (== (.itemid ArrayItem) (.itemid (Variables|/Game/Blueprints/Items/BP_ItemPickup.BP_ItemPickup_C|GetItemData _asbp_item_pickup)))
            (Default|AddQuantity _asbp_item_pickup 1)
            (LocalVariables|SetDroppedItemAlreadyNearby true)
            (goto _label Break)))
        (:Completed
          (if (LocalVariables|GetDroppedItemAlreadyNearby)
            _
            (else
              (bind _returnvalue_4 (Game|SpawnActorfromClass (LocalVariables|GetItemClassToSpawn) (Math|Transform|MakeTransform (+ _returnvalue_2 (* (Transformation|GetActorForwardVector _returnvalue) 1e+02))) "Undefined" "MultiplyWithRoot" 0 (Utilities|Struct|MakeST_ItemData _itemid 1) (Game|GetPlayerCharacter 0)))
              (Utilities|IsValid _returnvalue_4
                (:Is%20Valid
                  _))))
          (Utilities|Array|SetArrayElem (Variables|Default|GetInventoryItems) CurrentArrayIndex (Utilities|Struct|MakeST_ItemData _itemid (- _quantity 1)))
          (if (<= (Utilities|Array|Length (Variables|Default|GetInventoryItems)) 0)
            (Utilities|Array|RemoveIndex (Variables|Default|GetInventoryItems) CurrentArrayIndex)))))))

(fn DropAllItemsfromInventory
  (params (CurrentArrayIndex :type Integer))
  (LocalVariables|SetCurrentIndex CurrentArrayIndex)
  (bind _returnvalue (Utilities|GetDataTableRow "/Game/Blueprints/Data/DT_ItemDataTable.DT_ItemDataTable" (.ItemID (Utilities|Struct|BreakST_ItemData (Utilities|Array|Get(acopy) (Variables|Default|GetInventoryItems) (LocalVariables|GetCurrentIndex)))))
    (:then
      (bind _output_get (LocalVariables|SetItemClassToSpawn (.itempickupclass _returnvalue)))
      ;[0.15 0.15 0.15 0.5] Check For Item Already in world, if yes then add to its quantity instead of spawning a new one
      (bind _outactors (Collision|SphereOverlapActors (Transformation|GetActorLocation (Components|GetOwner)) 128.0 (LocalVariables|GetObjectTypeQuery) "/Game/Blueprints/Items/BP_ItemPickup.BP_ItemPickup_C"))
      (bind _array_element (Utilities|Array|ForEachLoopwithBreak _outactors :!label _label)
        (:LoopBody
          (bind _asbp_item_pickup (Utilities|Casting|CastToBP_ItemPickup _array_element))
          (if (== (.ItemID (Utilities|Struct|BreakST_ItemData (Utilities|Array|Get(acopy) (Variables|Default|GetInventoryItems) (LocalVariables|GetCurrentIndex)))) (.itemid (Variables|/Game/Blueprints/Items/BP_ItemPickup.BP_ItemPickup_C|GetItemData _asbp_item_pickup)))
            (Default|AddQuantity _asbp_item_pickup (.Quantity (Utilities|Struct|BreakST_ItemData (Utilities|Array|Get(acopy) (Variables|Default|GetInventoryItems) (LocalVariables|GetCurrentIndex)))))
            (LocalVariables|SetDroppedItemAlreadyNearby true)
            (goto _label Break)))
        (:Completed
          (if (LocalVariables|GetDroppedItemAlreadyNearby)
            _
            (else
              (bind _returnvalue_2 (Game|SpawnActorfromClass _output_get (CallFunction|GetPickupItemSpawnLocation) "Undefined" "MultiplyWithRoot" 0 (Utilities|Array|Get(acopy) (Variables|Default|GetInventoryItems) (LocalVariables|GetCurrentIndex)) (Game|GetPlayerCharacter 0)))
              (Utilities|IsValid _returnvalue_2
                (:Is%20Valid
                  _))))
          (Utilities|Array|RemoveIndex (Variables|Default|GetInventoryItems) (LocalVariables|GetCurrentIndex)))))))

(fn GetPickupItemSpawnLocation
  (bind _returnvalue (Components|GetOwner))
  (return (Math|Transform|MakeTransform (+ (Transformation|GetActorLocation _returnvalue) (* (Transformation|GetActorForwardVector _returnvalue) 1e+02)))))

(fn CheckandUseItemfromInventory
  (params (ItemID :type Name) (ItemUseQuantity :type Integer))
  (bind (_array_element _array_index) (Utilities|Array|ForEachLoopwithBreak (Variables|Default|GetInventoryItems) :!label _label)
    (:LoopBody
      (if (== (.ItemID (Utilities|Struct|BreakST_ItemData _array_element)) ItemID)
        (if (>= (.Quantity (Utilities|Struct|BreakST_ItemData _array_element)) ItemUseQuantity)
          (LocalVariables|SetItemUsedSuccessfully true)
          (if (== (.Quantity (Utilities|Struct|BreakST_ItemData _array_element)) ItemUseQuantity)
            (Utilities|Array|RemoveIndex (Variables|Default|GetInventoryItems) (LocalVariables|GetCurrentIndex))
            (Development|PrintString "Removed")
            (goto _label Break)
            (else
              (Utilities|Array|SetArrayElem (Variables|Default|GetInventoryItems) _array_index (Utilities|Struct|MakeST_ItemData (.ItemID (Utilities|Struct|BreakST_ItemData _array_element)) (- (.Quantity (Utilities|Struct|BreakST_ItemData _array_element)) ItemUseQuantity)))
              (Development|PrintString (Utilities|String|Append (Utilities|String|ToString(Name) (.ItemID (Utilities|Struct|BreakST_ItemData _array_element))) (Utilities|String|ToString(Integer) (- (.Quantity (Utilities|Struct|BreakST_ItemData _array_element)) ItemUseQuantity))))
              (goto _label Break))))))
    (:Completed
      (if (LocalVariables|GetItemUsedSuccessfully)
        (Default|CallOnInventoryChanged))
      (return (LocalVariables|GetItemUsedSuccessfully)))))