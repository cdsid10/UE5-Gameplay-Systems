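; BP_BaseDrink is the base actor for drinks that are consumed through interaction.
; On Interact, TryConsumeDrink looks for a BP_DrinkComponent on the interactor and, if it is valid, passes its DrinkData to that component's ConsumeDrink.
; The drink itself applies no effects, and EndInteraction is empty.
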(event EventBeginPlay
  (|CallParentFunction) ; This node is disabled and will not be called.\nDrag off pins to build functionality.
)

(event Collision|EventActorBeginOverlap
  (params (OtherActor :type Actor%20Object%20Reference))
  (|CallParentFunction OtherActor) ; This node is disabled and will not be called.\nDrag off pins to build functionality.
)

(event EventTick
  (params (DeltaSeconds :type Float%20%28single-precision%29))
  (|CallParentFunction DeltaSeconds) ; This node is disabled and will not be called.\nDrag off pins to build functionality.
)

(event EventInteract
  (params (Interactor :type BP%20Third%20Person%20Character%20Object%20Reference))
  (CallFunction|TryConsumeDrink Interactor))

(event EventEndInteraction
  (params (Interactor :type BP%20Third%20Person%20Character%20Object%20Reference)))

(fn ConstructionScript
  (|CallParentFunction))

(fn TryConsumeDrink
  (params (Interactor :type BP%20Third%20Person%20Character%20Object%20Reference))
  (bind _returnvalue (Actor|GetComponentbyClass Interactor "/Game/Blueprints/_Drink/Core/BP_DrinkComponent.BP_DrinkComponent_C"))
  (Utilities|IsValid _returnvalue
    (:Is%20Valid
      (if true
        (Default|ConsumeDrink _returnvalue (Variables|Default|GetDrinkData))))))