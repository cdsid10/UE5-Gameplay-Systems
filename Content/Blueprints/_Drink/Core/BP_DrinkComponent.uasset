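; Drink component that tracks alcohol intake, dizziness, drunk state and blackouts.
; ConsumeDrink adds alcohol scaled by remaining headroom and extends a sober delay; a looping timer runs that delay down, then decays alcohol while interpolating dizziness at separate rise and fall speeds.
; Threshold checks set the drunk state and a dispatcher broadcasts stat changes.
; High alcohol plus a long sober delay triggers blackout: camera fade, stats reset, delayed recovery.
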(event Custom|UpdateDrunkEffects
  (if (and (> (Variables|Alcohol|GetAlcoholLevel) 0.0) (not (Variables|BlackOut|GetIsBlackout)))
    (CallFunction|UpdateDrinkEffects)))

(event Custom|ResetBlackout
  (Utilities|FlowControl|Delay 5.0)
  (Variables|BlackOut|SetIsBlackout false)
  (CameraFades|StartCameraFade :self (Game|GetPlayerCameraManager 0) :FromAlpha 1.0 :Duration 0.5 :bHoldWhenFinished true)
  (CallFunction|SetDrunkState "NewEnumerator0")
  (Default|CallOnDrinkStatsChanged))

(event EventBeginPlay
  (EventDispatchers|BindEventtoOnResetBlackout (delegate Custom|ResetBlackout))
  (Utilities|Time|SetTimerbyEvent (delegate Custom|UpdateDrunkEffects) (Variables|Timers|GetUpdateInterval) true))

(fn ConsumeDrink
  (params (DrinkData :type ST%20Drink%20Data%20Structure))
  (bind (_drinkname _price _drinkstrength _drinkduration) (Utilities|Struct|BreakST_DrinkData DrinkData))
  (Development|PrintString (Utilities|String|Append "Consumed: " (Utilities|String|ToString(Name) (.drinkname DrinkData)) "!") true true "(R=1.000000,G=0.180842,B=0.000000,A=1.000000)")
  (Math|Integer|IncrementInt (Variables|Consumption|GetDrinksConsumed)
    (:%20%20
      (LocalVariables|SetEffectiveStrength (* (- (Variables|Alcohol|GetMaxAlcoholLevel) (Variables|Alcohol|GetAlcoholLevel)) _drinkstrength))
      (bind _output_get (Variables|Alcohol|SetAlcoholLevel (Math|Float|Clamp(Float) (+ (Variables|Alcohol|GetAlcoholLevel) (LocalVariables|GetEffectiveStrength)) 0.0 (Variables|Alcohol|GetMaxAlcoholLevel))))
      (Variables|Dizziness|SetTargetDizziness _output_get)
      (Variables|Timers|SetSoberDelayTimer (Math|Float|Clamp(Float) (+ (Variables|Timers|GetSoberDelayTimer) _drinkduration) 0.0 6e+01))
      (if (CallFunction|CheckBlackout)
        (CallFunction|TriggerBlackout)
        (else
          (bind _drunkstate (CallFunction|GetDrunkState))
          (CallFunction|SetDrunkState _drunkstate)))
      (Default|CallOnDrinkStatsChanged))))

(fn ApplyDrinkEffect)

(fn UpdateDizziness)

(fn GetDrunkState
  (if (<= (Variables|Alcohol|GetAlcoholLevel) 0.1)
    (return "NewEnumerator0")
    (elif (<= (Variables|Alcohol|GetAlcoholLevel) 0.3)
      (return "NewEnumerator5")
      (elif (<= (Variables|Alcohol|GetAlcoholLevel) 0.5)
        (return "NewEnumerator1")
        (elif (< (Variables|Alcohol|GetAlcoholLevel) 0.7)
          (return "NewEnumerator2")
          (else
            (if (< (Variables|Alcohol|GetAlcoholLevel) (Variables|BlackOut|GetBlackOutThreshold))
              _
              (else
                _))
            (return "NewEnumerator3")))))))

(fn SetDrinkWBP
  (params (DrinkStatusWidgetRef :type WBP%20Drink%20Status%20Object%20Reference))
  (Variables|WBPReference|SetDrinkStatusWidgetRef DrinkStatusWidgetRef))

(fn UpdateDrinkEffects
  (if (> (Variables|Timers|GetSoberDelayTimer) 0.0)
    (Variables|Timers|SetSoberDelayTimer (Math|Float|Max(Float) (- (Variables|Timers|GetSoberDelayTimer) (Variables|Timers|GetUpdateInterval)) 0.0))
    (else
      (bind _output_get (Variables|Alcohol|SetAlcoholLevel (- (Variables|Alcohol|GetAlcoholLevel) (* (Variables|Alcohol|GetAlcoholDecayRate) (Variables|Timers|GetUpdateInterval)))))
      (Variables|Dizziness|SetTargetDizziness _output_get)))
  (if (> (Variables|Dizziness|GetTargetDizziness) (Variables|Dizziness|GetCurrentDizziness))
    (Variables|Speeds|SetInterpSpeed (Variables|Speeds|GetBuildUpSpeed))
    (else
      (Variables|Speeds|SetInterpSpeed (Variables|Speeds|GetSoberDownSpeed))))
  (bind _output_get_2 (Variables|Dizziness|SetCurrentDizziness (Math|Float|Clamp(Float) (Math|Interpolation|FInterpTo (Variables|Dizziness|GetCurrentDizziness) (Variables|Dizziness|GetTargetDizziness) (Variables|Timers|GetUpdateInterval) (Variables|Speeds|GetInterpSpeed)) 0.0 (Variables|Dizziness|GetMaxDizziness))))
  (if (<= _output_get_2 0.035)
    (Variables|Dizziness|SetCurrentDizziness 0.0))
  (bind _drunkstate (CallFunction|GetDrunkState))
  (CallFunction|SetDrunkState _drunkstate)
  (Default|CallOnDrinkStatsChanged))

(fn SetDrunkState
  (params (DrunkState :type EDrunkState%20Enum :default "NewEnumerator0"))
  (Variables|DrinkDetails|SetDrunkState DrunkState))

(fn TriggerBlackout
  (Variables|BlackOut|SetIsBlackout true)
  (CallFunction|SetDrunkState "NewEnumerator4")
  (Default|CallOnDrinkStatsChanged)
  (CameraFades|StartCameraFade :self (Game|GetPlayerCameraManager 0) :ToAlpha 1.0 :Duration 0.5 :bHoldWhenFinished true)
  (Development|PrintString "PLAYER BLACKED OUT!" true true "(R=1.000000,G=0.000334,B=0.000007,A=1.000000)" 5.0)
  (Variables|Alcohol|SetAlcoholLevel 0.0)
  (Variables|Dizziness|SetTargetDizziness 0.0)
  (Variables|Dizziness|SetCurrentDizziness 0.0)
  (Variables|Timers|SetSoberDelayTimer 0.0)
  (Default|CallOnResetBlackout))

(fn CheckBlackout
  (return (Math|Boolean|ANDBoolean (>= (Variables|Alcohol|GetAlcoholLevel) (Variables|BlackOut|GetBlackOutThreshold)) (> (Variables|Timers|GetSoberDelayTimer) 3e+01) (not (Variables|BlackOut|GetIsBlackout)))))