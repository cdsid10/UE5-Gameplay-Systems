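; BP_FastTravelPoint represents a fast travel destination and caches that destination's data.
; LoadDestinationData converts the DestinationID enum to a row name, looks it up in DestinationDataTable and stores the row in CachedDestinationData.
; The lookup runs in both the construction script and BeginPlay, printing a warning when the row is missing.
; It contains no overlap, tick or travel logic.
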(event EventBeginPlay
  (CallFunction|LoadDestinationData))

(event Collision|EventActorBeginOverlap
  (params (OtherActor :type Actor%20Object%20Reference)))

(event EventTick
  (params (DeltaSeconds :type Float%20%28single-precision%29)))

(fn ConstructionScript
  (CallFunction|LoadDestinationData))

(fn LoadDestinationData
  (bind _returnvalue (Utilities|GetDataTableRow (Variables|TravelPointData|GetDestinationDataTable) (Utilities|String|StringToName (Utilities|String|EnumtoString (Variables|TravelPointData|GetDestinationID))))
    (:then
      (Variables|TravelPointData|SetCachedDestinationData _returnvalue))
    (:RowNotFound
      (Development|PrintString "Missing Fast Travel Data for DestinationID"))))