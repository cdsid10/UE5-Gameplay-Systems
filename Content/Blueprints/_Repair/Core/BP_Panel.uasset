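; BP_Panel is a repair piece that slides open when its repair interaction plays.
; The interaction override calls an event dispatcher, bound on BeginPlay, to reach the timeline in the event graph from a function.
; The timeline adds its slide value as a Z offset to the root every update, so movement accumulates.
; On completion it prints a debug message and finishes the repair step with the passed target state.
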(event Custom|OpenPanelEvent
  (params (TargetState :type ERepairState%20Enum :default "NewEnumerator0"))
  (bind _panelslide (Timeline|OpenPanelTimeline Play)
    (:Update
      (Transformation|AddRelativeLocation (Variables|Default|GetDefaultSceneRoot) (Math|Vector|MakeVector 0.0 0.0 _panelslide) false false))
    (:Finished
      (Development|PrintString "Finsihed Opening")
      (CallFunction|FinishRepairStep TargetState))))

(event EventBeginPlay
  (|CallParentFunction)
  (EventDispatchers|BindEventtoStartOpenPanelTimeline (delegate Custom|OpenPanelEvent)))

(fn ConstructionScript
  (|CallParentFunction))

(fn PlayRepairPieceInteraction
  (params (TargetState :type ERepairState%20Enum :default "NewEnumerator0"))
  (CallFunction|PlayOpenAnimation TargetState))

(fn PlayOpenAnimation
  (params (TargetState :type ERepairState%20Enum :default "NewEnumerator0"))
  (Default|CallStartOpenPanelTimeline TargetState))