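; Repair piece that tracks its repair state as one part of an owning repairable object, apparently serving as a base for specific pieces.
; ApplyRepairStep calls an empty PlayRepairPieceInteraction hook and prints target and current states; its FinishRepairStep call is disconnected.
; FinishRepairStep, when called, commits the new state and notifies the owner.
; Highlighting toggles an overlay material on the interactable mesh.
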(event EventBeginPlay
  (CallFunction|Initialize))

(fn ConstructionScript)

(fn PlayRepairPieceInteraction
  (params (TargetState :type ERepairState%20Enum :default "NewEnumerator0")))

(fn ApplyRepairStep
  (params (TargetState :type ERepairState%20Enum :default "NewEnumerator0"))
  (CallFunction|PlayRepairPieceInteraction TargetState)
  (Development|PrintString (Utilities|String|Append "Target State: " (Utilities|String|EnumtoString TargetState) " " "Current State: " (Utilities|String|EnumtoString (Variables|RepairPieceData|GetCurrentState)))))

(fn Initialize
  (Variables|RepairPieceData|SetCurrentState (Variables|RepairPieceData|GetDefaultState)))

(fn GetCurrentState
  (return (Variables|RepairPieceData|GetCurrentState)))

(fn SetCurrentState
  (params (NewState :type ERepairState%20Enum :default "NewEnumerator0"))
  (Variables|RepairPieceData|SetCurrentState NewState))

(fn FinishRepairStep
  (params (TargetRepairState :type ERepairState%20Enum :default "NewEnumerator0"))
  (Variables|RepairPieceData|SetCurrentState TargetRepairState)
  (Default|NotifyRepairPieceFinished (Variables|RepairPieceData|GetOwnerRepairable)))

(fn SetOwnerRepairable
  (params (OwnerRepairableObject :type BP%20Repairable%20Object%20Object%20Reference))
  (Variables|RepairPieceData|SetOwnerRepairable OwnerRepairableObject))

(fn SetHighlighted
  (params (IsHighlighted :type Boolean))
  (if IsHighlighted
    (Rendering|Material|SetOverlayMaterial (Variables|Default|GetInteractableMesh) "/Engine/BasicShapes/OverlayMaterial.OverlayMaterial" :!class /Script/Engine.MeshComponent)
    (else
      (Rendering|Material|SetOverlayMaterial (Variables|Default|GetInteractableMesh) 0 :!class /Script/Engine.MeshComponent))))