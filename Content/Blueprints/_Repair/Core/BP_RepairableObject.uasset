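; Repairable world object that players fix through an ordered list of repair steps.
; On BeginPlay it registers nearby repair pieces by sphere overlap; interacting opens the repair menu and enters the player's repair mode.
; StartRepair attaches pieces to YawPivot, then highlights each step's piece, gating clicks through Visibility collision.
; Valid piece, state and tool, plus any required inventory item, apply the step; piece notifications advance it until pieces detach and repair mode exits.
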(event EventBeginPlay
  (bind _outactors (Collision|SphereOverlapActors (Transformation|GetWorldLocation (Variables|Default|GetBaseMesh)) 32.0 (Variables|RepairData|GetRepairPieceObjectTypesQuery) "/Game/Blueprints/_Repair/Core/BP_RepairPiece.BP_RepairPiece_C"))
  (for _array_element _outactors
    (bind _asbp_repair_piece (Utilities|Casting|CastToBP_RepairPiece _array_element))
    (Default|SetOwnerRepairable _asbp_repair_piece self)
    (CallFunction|AddtoRepairPiecesArray _asbp_repair_piece)
    (Collision|SetCollisionResponsetoChannel (Variables|/Game/Blueprints/_Repair/Core/BP_RepairPiece.BP_RepairPiece_C|GetInteractableMesh _asbp_repair_piece) "ECC_Visibility" "ECR_Ignore")))

(event Collision|EventActorBeginOverlap
  (params (OtherActor :type Actor%20Object%20Reference)))

(event EventTick
  (params (DeltaSeconds :type Float%20%28single-precision%29)))

(event EventInteract
  (params (Interactor :type BP%20Third%20Person%20Character%20Object%20Reference))
  (bind _returnvalue (Actor|GetComponentbyClass Interactor "/Game/Blueprints/Inventory/BP_InventoryComponent.BP_InventoryComponent_C"))
  (bind _returnvalue_2 (Actor|GetComponentbyClass Interactor "/Game/Blueprints/_Repair/Player/BP_RepairComponent.BP_RepairComponent_C"))
  (Utilities|IsValid _returnvalue
    (:Is%20Valid
      (Variables|Default|SetPlayerInventoryComponent _returnvalue)
      (Default|OpenCloseRepairMenu Interactor)
      (Utilities|IsValid _returnvalue_2
        (:Is%20Valid
          (bind _output_get (Variables|Default|SetPlayerRepairComponent _returnvalue_2))
          (Default|EnterRepairMode _output_get self))))))

(event EventEndInteraction
  (params (Interactor :type BP%20Third%20Person%20Character%20Object%20Reference))
  (bind _returnvalue (Actor|GetComponentbyClass Interactor "/Game/Blueprints/_Repair/Player/BP_RepairComponent.BP_RepairComponent_C"))
  (if (Variables|/Game/ThirdPerson/Blueprints/BP_ThirdPersonCharacter.BP_ThirdPersonCharacter_C|GetCanInteract Interactor)
    (Default|OpenCloseRepairMenu Interactor)
    (Utilities|IsValid _returnvalue
      (:Is%20Valid
        (Default|ExitRepairMode _returnvalue)))))

(fn ConstructionScript)

(fn ProcessInteraction
  (params (ClickedRepairPiece :type BP%20Repair%20Piece%20Object%20Reference) (SelectedTool :type ERepairTool%20Enum :default "NewEnumerator0"))
  (bind _currentactivestep (Variables|RepairData|GetCurrentActiveStep))
  (bind (_repairpiecereference _requiredtool _requiredstate _targetstate _instruction _interactionduration _requiresinventoryitem_ _inventoryitemid _inventoryitemusequantity) (Utilities|Struct|BreakST_RepairStep _currentactivestep))
  (if (CallFunction|CanPerformStep ClickedRepairPiece SelectedTool)
    (if _requiresinventoryitem_
      (bind _coulduseitem (Default|CheckandUseItemfromInventory (Variables|Default|GetPlayerInventoryComponent) _inventoryitemid _inventoryitemusequantity))
      (if _coulduseitem
        (CallFunction|PerformStep :!label _label)
        (else
          (Development|PrintString "Not enough items in invenotry")))
      (else
        (Development|PrintString (Utilities|String|Append (Utilities|GetDisplayName ClickedRepairPiece) ""))
        (goto _label)))
    (else
      (Development|PrintString (Utilities|String|Append (Utilities|GetDisplayName ClickedRepairPiece) " WITH TOOL SELECTED: " (Utilities|String|EnumtoString SelectedTool) " SOMETHING IS WRONG")))))

(fn GetCurrentStep
  (return (Utilities|Array|Get(acopy) (Variables|RepairData|GetRepairSteps) (Variables|RepairData|GetCurrentStepIndex))))

(fn CanPerformStep
  (params (ClickedRepairPiece :type BP%20Repair%20Piece%20Object%20Reference) (SelectedTool :type ERepairTool%20Enum :default "NewEnumerator0"))
  (bind _currentactivestep (Variables|RepairData|GetCurrentActiveStep))
  (bind (_repairpiecereference _requiredtool _requiredstate) (Utilities|Struct|BreakST_RepairStep _currentactivestep))
  (return (Math|Boolean|ANDBoolean (== ClickedRepairPiece _repairpiecereference) (Utilities|Enum|Equal(Enum) (Default|GetCurrentState ClickedRepairPiece) _requiredstate) (Utilities|Enum|Equal(Enum) SelectedTool _requiredtool))))

(fn PerformStep
  (bind _currentactivestep (Variables|RepairData|GetCurrentActiveStep))
  (bind (_repairpiecereference _requiredtool _requiredstate _targetstate) (Utilities|Struct|BreakST_RepairStep _currentactivestep))
  (Default|ApplyRepairStep _repairpiecereference _targetstate))

(fn StartRepair
  (CallFunction|AttachRepairPieces)
  (Variables|RepairData|SetIsRepairFinished false)
  (Variables|RepairData|SetCurrentStepIndex 0)
  (Collision|SetCollisionResponsetoChannel (Variables|Default|GetBox_Collision) "ECC_Visibility" "ECR_Ignore")
  (Collision|SetCollisionResponsetoChannel (Variables|Default|GetBaseMesh) "ECC_Visibility" "ECR_Ignore")
  (CallFunction|ActivateCurrentStep))

(fn ActivateCurrentStep
  (if (>= (Variables|RepairData|GetCurrentStepIndex) (Utilities|Array|Length (Variables|RepairData|GetRepairSteps)))
    (CallFunction|FinishRepair)
    (else
      (bind _output_get (Variables|RepairData|SetCurrentActiveStep (Utilities|Array|Get(acopy) (Variables|RepairData|GetRepairSteps) (Variables|RepairData|GetCurrentStepIndex))))
      (Development|PrintString (Utilities|String|Append "Current Active Piece is: " (Utilities|GetDisplayName (.RepairPieceReference (Utilities|Struct|BreakST_RepairStep _output_get)))))
      (Collision|SetCollisionResponsetoChannel (Variables|/Game/Blueprints/_Repair/Core/BP_RepairPiece.BP_RepairPiece_C|GetInteractableMesh (.RepairPieceReference (Utilities|Struct|BreakST_RepairStep _output_get))) "ECC_Visibility" "ECR_Block")
      (Default|SetHighlighted (.RepairPieceReference (Utilities|Struct|BreakST_RepairStep _output_get)) true)
      (Development|PrintString (Utilities|String|Append "Current Object with block channel is: " (Utilities|GetDisplayName (Variables|/Game/Blueprints/_Repair/Core/BP_RepairPiece.BP_RepairPiece_C|GetInteractableMesh (.RepairPieceReference (Utilities|Struct|BreakST_RepairStep _output_get)))))))))

(fn FinishRepair
  (Development|PrintString "Repair is Finished!" true true "(R=0.377756,G=0.000000,B=1.000000,A=1.000000)")
  (Variables|RepairData|SetIsRepairFinished true)
  (Variables|RepairData|SetCurrentActiveStep "")
  (CallFunction|DetachRepairPieces)
  (Default|ExitRepairMode (Variables|Default|GetPlayerRepairComponent)))

(fn AdvanceStep
  (bind _currentactivestep (Variables|RepairData|GetCurrentActiveStep))
  (bind _currentstepindex (Variables|RepairData|GetCurrentStepIndex))
  (bind _repairsteps (Variables|RepairData|GetRepairSteps))
  (bind _repairpiecereference (Utilities|Struct|BreakST_RepairStep _currentactivestep))
  (bind _returnvalue (Utilities|Array|Length _repairsteps))
  (Utilities|IsValid _repairpiecereference
    (:Is%20Valid
      (Default|SetHighlighted _repairpiecereference false)
      (Collision|SetCollisionResponsetoChannel (Variables|/Game/Blueprints/_Repair/Core/BP_RepairPiece.BP_RepairPiece_C|GetInteractableMesh _repairpiecereference) "ECC_Visibility" "ECR_Ignore")
      (Math|Integer|IncrementInt (Variables|RepairData|GetCurrentStepIndex)
        (:%20%20
          (Development|PrintString (Utilities|String|Append "Current Step: " (Utilities|String|ToString(Integer) _currentstepindex) " & " "Repair Steps Length: " (Utilities|String|ToString(Integer) _returnvalue)) true true "(R=1.000000,G=0.634525,B=0.000000,A=1.000000)")
          (if (>= _currentstepindex _returnvalue)
            (CallFunction|FinishRepair)
            (else
              (CallFunction|ActivateCurrentStep))))))))

(fn NotifyRepairPieceFinished
  (CallFunction|AdvanceStep))

(fn AttachRepairPieces
  (for _array_element (Variables|RepairData|GetRepairPieces)
    (Utilities|IsValid _array_element
      (:Is%20Valid
        (Transformation|AttachComponentToComponent _array_element (Variables|Default|GetYawPivot) "None" "KeepWorld" "KeepWorld" "KeepWorld" false)))))

(fn DetachRepairPieces
  (for _array_element (Variables|RepairData|GetRepairPieces)
    (Utilities|IsValid _array_element
      (:Is%20Valid
        (Transformation|DetachFromActor _array_element "KeepWorld" "KeepWorld" "KeepWorld")))))

(fn AddtoRepairPiecesArray
  (params (CurrentRepairPiece :type BP%20Repair%20Piece%20Object%20Reference))
  (Utilities|Array|AddUnique (Variables|RepairData|GetRepairPieces) CurrentRepairPiece))