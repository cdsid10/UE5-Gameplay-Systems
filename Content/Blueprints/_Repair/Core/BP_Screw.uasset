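; Screw repair piece that animates being unscrewed or screwed in as a step of the repair interaction.
; The PlayRepairPieceInteraction override calls RotateScrew, which picks a direction from the target state and fires the matching event dispatcher, bound on BeginPlay.
; Each bound event plays a timeline that adds relative Z offsets to the root, with no actual rotation, then finishes the repair step with that state.
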(event Custom|UnscrewEvent
  (params (TargetState :type ERepairState%20Enum :default "NewEnumerator0"))
  (bind _scale (Timeline|UnscrewTimeline Play)
    (:Update
      (Transformation|AddRelativeLocation (Variables|Default|GetDefaultSceneRoot) (Math|Vector|MakeVector 0.0 0.0 _scale) false false))
    (:Finished
      (Development|PrintString "Finsihed Unscrewing")
      (CallFunction|FinishRepairStep TargetState))))

(event Custom|ScrewEvent
  (params (TargetState :type ERepairState%20Enum :default "NewEnumerator0"))
  (bind _scale (Timeline|ScrewTimeline Play)
    (:Update
      (Transformation|AddRelativeLocation (Variables|Default|GetDefaultSceneRoot) (Math|Vector|MakeVector 0.0 0.0 _scale) false false))
    (:Finished
      (Development|PrintString "Finsihed Screwing")
      (CallFunction|FinishRepairStep TargetState))))

(event EventBeginPlay
  (|CallParentFunction)
  (EventDispatchers|BindEventtoStartUnscrewTimeline (delegate Custom|UnscrewEvent))
  (EventDispatchers|BindEventtoStartScrewTimeline (delegate Custom|ScrewEvent)))

(fn ConstructionScript
  (|CallParentFunction))

(fn PlayRepairPieceInteraction
  (params (TargetState :type ERepairState%20Enum :default "NewEnumerator0"))
  (CallFunction|RotateScrew TargetState))

(fn RotateScrew
  (params (TargetState :type ERepairState%20Enum :default "NewEnumerator0"))
  (if (Utilities|Enum|Equal(Enum) TargetState "NewEnumerator0")
    (Default|CallStartUnscrewTimeline TargetState)
    (else
      (Default|CallStartScrewTimeline TargetState))))