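; Repair piece for a phone back cover that slides off and back on during repairs.
; Interaction dispatches open or close from the current Installed or Removed state, swapping to a hidden animatable mesh that timelines lerp between its resting position and a slide-up target.
; When opening finishes, the cover hides and goes into the player's inventory; both directions then finish the repair step.
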(event Custom|OpenBackCover
  (params (TargetState :type ERepairState%20Enum :default "NewEnumerator0"))
  (Development|SetHiddeninGame (Variables|Default|GetInteractableMesh) true false)
  (Development|SetHiddeninGame (Variables|Default|GetAnimateableMesh) false false)
  (Variables|Default|SetStartLocation (Variables|/Script/Engine.SceneComponent|GetRelativeLocation (Variables|Default|GetInteractableMeshParent)))
  (Variables|Default|SetEndLocation (Variables|/Script/Engine.SceneComponent|GetRelativeLocation (Variables|Default|GetSlideUpTarget)))
  (bind _slideupalpha (Timeline|OpenBackCoverTimeline Play)
    (:Update
      (Transformation|SetRelativeLocation (Variables|Default|GetAnimateableMeshParent) (Math|Vector|Lerp(Vector) (Variables|Default|GetStartLocation) (Variables|Default|GetEndLocation) _slideupalpha) false false))
    (:Finished
      (Development|SetHiddeninGame (Variables|Default|GetAnimateableMesh) true false)
      (Default|AddItem (Variables|/Game/Blueprints/_Repair/Core/BP_RepairableObject.BP_RepairableObject_C|GetPlayerInventoryComponent (Variables|Default|GetOwnerRepairable)) (Utilities|Struct|MakeST_ItemData (Variables|Default|GetInventoryItemID) 1))
      (CallFunction|FinishRepairStep TargetState))))

(event Custom|CloseBackCover
  (params (TargetState :type ERepairState%20Enum :default "NewEnumerator0"))
  (Development|SetHiddeninGame (Variables|Default|GetAnimateableMesh) false false)
  (bind _slideupalpha (Timeline|CloseBackCoverTimeline Play)
    (:Update
      (Transformation|SetRelativeLocation (Variables|Default|GetAnimateableMeshParent) (Math|Vector|Lerp(Vector) (Variables|Default|GetEndLocation) (Variables|Default|GetStartLocation) _slideupalpha) false false))
    (:Finished
      (CallFunction|FinishRepairStep TargetState))))

(event EventBeginPlay
  (|CallParentFunction)
  (EventDispatchers|BindEventtoOnOpenBackCover (delegate Custom|OpenBackCover))
  (EventDispatchers|BindEventtoOnCloseBackCover (delegate Custom|CloseBackCover))
  (Development|SetHiddeninGame (Variables|Default|GetAnimateableMesh) true false))

(fn ConstructionScript
  (|CallParentFunction))

(fn PlayRepairPieceInteraction
  (params (TargetState :type ERepairState%20Enum :default "NewEnumerator0"))
  (switch Utilities|FlowControl|Switch|SwitchonERepairState (CallFunction|GetCurrentState)
    (:NewEnumerator0
      (Default|CallOnOpenBackCover TargetState))
    (:NewEnumerator1
      (Default|CallOnCloseBackCover TargetState))))

(fn SetStartandEndTransforms
  (Variables|Default|SetStartLocation (Variables|/Script/Engine.SceneComponent|GetRelativeLocation (Variables|Default|GetAnimateableMeshParent)))
  (Variables|Default|SetEndLocation (Variables|/Script/Engine.SceneComponent|GetRelativeLocation (Variables|Default|GetMoveAwayTarget)))
  (Variables|Default|SetStartRotation (Variables|/Script/Engine.SceneComponent|GetRelativeRotation (Variables|Default|GetAnimateableMeshParent)))
  (Variables|Default|SetEndRotation "0, 0, 0"))