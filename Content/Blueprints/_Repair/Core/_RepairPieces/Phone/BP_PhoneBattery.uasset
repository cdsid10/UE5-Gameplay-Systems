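; Phone battery repair piece that animates a battery swap when the player performs its repair interaction.
; The interaction fires an event dispatcher that swaps the interactable mesh for an animated one and captures start and target transforms.
; A removal timeline lerps the mesh's parent between them, then the mesh hides briefly before an insert timeline animates the installation.
; The repair step finishes once insertion completes.
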(event Custom|RemoveBattery
  (params (TargetState :type ERepairState%20Enum :default "NewEnumerator0"))
  (Development|SetHiddeninGame (Variables|Default|GetInteractableMesh) true false)
  (Development|SetHiddeninGame (Variables|Default|GetAnimateableMesh) false false)
  (CallFunction|SetStartandEndTransforms)
  (bind (_direction _removemovealpha _removerotationalpha) (Timeline|RemoveBatteryTimeline Play)
    (:Update
      (Transformation|SetRelativeRotation (Variables|Default|GetAnimateableMeshParent) (Math|Rotator|Lerp(Rotator) (Variables|Default|GetStartRotation) (Variables|Default|GetEndRotation) _removerotationalpha) false false)
      (Transformation|SetRelativeLocation (Variables|Default|GetAnimateableMeshParent) (Math|Vector|Lerp(Vector) (Variables|Default|GetStartLocation) (Variables|Default|GetEndLocation) _removemovealpha) false false))
    (:Finished
      (Development|SetHiddeninGame (Variables|Default|GetAnimateableMesh) true false)
      (Utilities|FlowControl|Delay 0.5)
      (Development|SetHiddeninGame (Variables|Default|GetAnimateableMesh) false false)
      (bind (_direction_2 _installmovealpha _installrotationalpha) (Timeline|InsertBatteryTimeline Play)
        (:Update
          (Transformation|SetRelativeRotation (Variables|Default|GetAnimateableMeshParent) (Math|Rotator|Lerp(Rotator) (Variables|Default|GetStartRotation) (Variables|Default|GetEndRotation) _installrotationalpha) false false)
          (Transformation|SetRelativeLocation (Variables|Default|GetAnimateableMeshParent) (Math|Vector|Lerp(Vector) (Variables|Default|GetStartLocation) (Variables|Default|GetEndLocation) _installmovealpha) false false))
        (:Finished
          (CallFunction|FinishRepairStep TargetState))))))

(event EventBeginPlay
  (|CallParentFunction)
  (EventDispatchers|BindEventtoOnRemoveBattery (delegate Custom|RemoveBattery))
  (Development|SetHiddeninGame (Variables|Default|GetAnimateableMesh) true false))

(fn ConstructionScript
  (|CallParentFunction))

(fn PlayRepairPieceInteraction
  (params (TargetState :type ERepairState%20Enum :default "NewEnumerator0"))
  (Default|CallOnRemoveBattery TargetState))

(fn SetStartandEndTransforms
  (Variables|Default|SetStartLocation (Variables|/Script/Engine.SceneComponent|GetRelativeLocation (Variables|Default|GetAnimateableMeshParent)))
  (Variables|Default|SetEndLocation (Variables|/Script/Engine.SceneComponent|GetRelativeLocation (Variables|Default|GetRemoveMoveTarget)))
  (Variables|Default|SetStartRotation (Variables|/Script/Engine.SceneComponent|GetRelativeRotation (Variables|Default|GetAnimateableMeshParent)))
  (Variables|Default|SetEndRotation (Variables|/Script/Engine.SceneComponent|GetRelativeRotation (Variables|Default|GetRemoveRotationTarget))))