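; BP_PhoneFrontCover is a phone repair piece for the front cover, which moves away and disappears when interacted with.
; PlayRepairPieceInteraction calls the OnOpenFrontCover dispatcher, which the piece binds to its own OpenFrontCover event on BeginPlay.
; A timeline adds its MoveAway value to the root's relative Y location on each update, so movement accumulates.
; When the timeline finishes, the actor is hidden and FinishRepairStep receives the target state.
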(event Custom|OpenFrontCover
  (params (TargetState :type ERepairState%20Enum :default "NewEnumerator0"))
  (bind _moveaway (Timeline|OpenFrontCoverTimeline Play)
    (:Update
      (Transformation|AddRelativeLocation (Variables|Default|GetDefaultSceneRoot) (Math|Vector|MakeVector 0.0 _moveaway 0.0) false false))
    (:Finished
      (Rendering|SetActorHiddenInGame true)
      (CallFunction|FinishRepairStep TargetState))))

(event EventBeginPlay
  (|CallParentFunction)
  (EventDispatchers|BindEventtoOnOpenFrontCover (delegate Custom|OpenFrontCover)))

(fn ConstructionScript
  (|CallParentFunction))

(fn PlayRepairPieceInteraction
  (params (TargetState :type ERepairState%20Enum :default "NewEnumerator0"))
  (Default|CallOnOpenFrontCover TargetState))