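; Repair piece for a phone's inner keypad that swaps the damaged keypad for a repaired one.
; The interaction override checks and consumes the active repair step's required inventory item, then fires the OnInnerKeypadReplaced dispatcher.
; The piece's own handler runs a timeline that nudges the damaged mesh along local Y, adding an offset each update.
; When the timeline finishes, it hides that mesh and reveals the initially hidden repaired mesh.
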(event Custom|KeypadReplaced
  (params (TargetState :type ERepairState%20Enum :default "NewEnumerator0"))
  (bind _moveaway (Timeline|DamagedKeypadTimeline Play)
    (:Update
      (Transformation|AddRelativeLocation (Variables|Default|GetInteractableMesh) (Math|Vector|MakeVector 0.0 _moveaway 0.0) false false))
    (:Finished
      (Development|SetHiddeninGame (Variables|Default|GetInteractableMesh) true false)
      (Development|SetHiddeninGame (Variables|Default|GetRepairedMesh) false false))))

(event EventBeginPlay
  (|CallParentFunction)
  (EventDispatchers|BindEventtoOnInnerKeypadReplaced (delegate Custom|KeypadReplaced))
  (Development|SetHiddeninGame (Variables|Default|GetRepairedMesh) true false))

(fn ConstructionScript
  (|CallParentFunction))

(fn PlayRepairPieceInteraction
  (params (TargetState :type ERepairState%20Enum :default "NewEnumerator0"))
  (bind _ownerrepairable (Variables|Default|GetOwnerRepairable))
  (bind _currentactivestep (Variables|/Game/Blueprints/_Repair/Core/BP_RepairableObject.BP_RepairableObject_C|GetCurrentActiveStep _ownerrepairable))
  (bind (_repairpiecereference _requiredtool _requiredstate _targetstate _instruction _interactionduration _requiresinventoryitem_ _inventoryitemid _inventoryitemusequantity) (Utilities|Struct|BreakST_RepairStep _currentactivestep))
  (bind _coulduseitem (Default|CheckandUseItemfromInventory (Variables|/Game/Blueprints/_Repair/Core/BP_RepairableObject.BP_RepairableObject_C|GetPlayerInventoryComponent _ownerrepairable) _inventoryitemid _inventoryitemusequantity))
  (if _coulduseitem
    (Default|CallOnInnerKeypadReplaced TargetState)))