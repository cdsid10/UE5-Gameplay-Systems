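; Player component on the third-person character that runs repair mode for repairable objects.
; Entering blends the camera to the repairable, hands it the repair widget and starts the repair; exiting blends back to the pawn.
; Holding right mouse rotates the repairable's YawPivot by yaw and clamped pitch.
; Clicks multi-trace under the cursor and pass the selected tool to the repairable only for the active step's piece.
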(event EventBeginPlay
  (bind _asplayer_controller (CallFunction|GetPlayerController))
  (Variables|Default|SetPlayerController _asplayer_controller))

(event EventTick
  (params (DeltaSeconds :type Float%20%28single-precision%29)))

(event Input|MouseEvents|MouseX
  (params (AxisValue :type Float%20%28single-precision%29))
  (if (Variables|Default|GetIsRotating)
    (Variables|Default|SetCurrentYaw (- (Variables|Default|GetCurrentYaw) (* AxisValue (Variables|Default|GetRotationSpeed))))
    (CallFunction|UpdateRotation)))

(event Input|MouseEvents|MouseY
  (params (AxisValue :type Float%20%28single-precision%29))
  (if (Variables|Default|GetIsRotating)
    (Variables|Default|SetCurrentPitch (Math|Float|Clamp(Float) (- (Variables|Default|GetCurrentPitch) (* AxisValue (Variables|Default|GetRotationSpeed))) -8e+01 8e+01))))

(event Input|MouseEvents|RightMouseButton
  (params (Key :type Key%20Structure))
  (:Pressed
    (if (Variables|Repair|GetIsRepairing)
      (Variables|Default|SetIsRotating true)))
  (:Released
    (if (Variables|Repair|GetIsRepairing)
      (Variables|Default|SetIsRotating false))))

(fn SetRepairableReference
  (params (RepairableReference :type BP%20Repairable%20Object%20Object%20Reference))
  (bind _output_get (Variables|Repair|SetCurrentRepairable RepairableReference))
  (Default|SetRepairWidget _output_get (Variables|Default|GetRepairWidgetReference))
  (return))

(fn EnterRepairMode
  (params (RepairableReference :type BP%20Repairable%20Object%20Object%20Reference))
  (CallFunction|SetRepairableReference RepairableReference)
  (Game|Player|SetViewTargetwithBlend (Variables|Default|GetPlayerController) RepairableReference 0.5 "VTBlend_Cubic" 0.0 false)
  (Variables|Repair|SetIsRepairing true)
  (Default|StartRepair RepairableReference)
  (Development|PrintString (Utilities|String|Append "Current Repair Tool: " (Utilities|String|EnumtoString (Variables|Repair|GetCurrentRepairTool)))))

(fn ExitRepairMode
  (bind _playercontroller (Variables|Default|GetPlayerController))
  (Game|Player|SetViewTargetwithBlend _playercontroller (Pawn|GetControlledPawn _playercontroller) 0.5 "VTBlend_Cubic" 0.0 false)
  (Variables|Repair|SetIsRepairing false)
  (Variables|Repair|SetCurrentRepairable 0))

(fn RepairClick
  (bind _returnvalue (Game|GetPlayerController 0))
  (bind (_worldlocation _worlddirection) (Game|Player|ConvertMouseLocationToWorldSpace _returnvalue))
  (if (Variables|Repair|GetIsRepairing)
    (bind _outhits (Collision|MultiLineTraceByChannel _worldlocation (+ _worldlocation (* _worlddirection 5e+03)) "TraceTypeQuery1" true 0 "ForOneFrame"))
    (bind _array_element (Utilities|Array|ForEachLoopwithBreak _outhits :!label _label)
      (:LoopBody
        (bind _asbp_repair_piece (Utilities|Casting|CastToBP_RepairPiece (.HitActor (Collision|BreakHitResult _array_element))))
        (if (== (.RepairPieceReference (Utilities|Struct|BreakST_RepairStep (Variables|/Game/Blueprints/_Repair/Core/BP_RepairableObject.BP_RepairableObject_C|GetCurrentActiveStep (Variables|/Game/Blueprints/_Repair/Core/BP_RepairPiece.BP_RepairPiece_C|GetOwnerRepairable _asbp_repair_piece)))) _asbp_repair_piece)
          (Default|ProcessInteraction (Variables|/Game/Blueprints/_Repair/Core/BP_RepairPiece.BP_RepairPiece_C|GetOwnerRepairable _asbp_repair_piece) _asbp_repair_piece (Variables|Repair|GetCurrentRepairTool))
          (goto _label Break))))))

(fn GetPlayerController
  (bind _asbp_third_person_character (Utilities|Casting|CastToBP_ThirdPersonCharacter (Components|GetOwner)))
  (bind _asplayer_controller (Utilities|Casting|CastToPlayerController (Pawn|GetController _asbp_third_person_character)))
  (return _asplayer_controller))

(fn SelectTool
  (params (ToolToSelect :type ERepairTool%20Enum :default "NewEnumerator0"))
  (Variables|Repair|SetCurrentRepairTool ToolToSelect))

(fn GetCurrentTool
  (return (Variables|Repair|GetCurrentRepairTool)))

(fn UpdateRotation
  (Transformation|SetRelativeRotation (Variables|/Game/Blueprints/_Repair/Core/BP_RepairableObject.BP_RepairableObject_C|GetYawPivot (Variables|Repair|GetCurrentRepairable)) (Math|Rotator|MakeRotator 0.0 (Variables|Default|GetCurrentPitch) (Variables|Default|GetCurrentYaw)) false false))