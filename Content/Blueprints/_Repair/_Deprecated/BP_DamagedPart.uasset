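; BP_DamagedPart is a deprecated repairable piece that the player replaces using items from their inventory.
; It starts showing the damaged StaticMesh, with RepairedMesh hidden.
; Repair, which overrides the parent without calling it, spends RepairCost of ItemID through the player's BP_InventoryComponent.
; On success it disables interaction, notifies the owning repairable item and swaps mesh visibility; otherwise it prints a failure message.
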(event EventBeginPlay
  (|CallParentFunction)
  (CallFunction|SetRepairedMeshState false))

(event Collision|EventActorBeginOverlap
  (params (OtherActor :type Actor%20Object%20Reference))
  (|CallParentFunction OtherActor) ; This node is disabled and will not be called.\nDrag off pins to build functionality.
)

(event EventTick
  (params (DeltaSeconds :type Float%20%28single-precision%29))
  (|CallParentFunction DeltaSeconds) ; This node is disabled and will not be called.\nDrag off pins to build functionality.
)

(fn ConstructionScript
  (|CallParentFunction))

(fn Repair
  (if (not (Variables|Default|GetIsCompleted))
    (bind _coulduseitem (Default|CheckandUseItemfromInventory (Actor|GetComponentbyClass (Variables|Default|GetPlayerCharacter) "/Game/Blueprints/Inventory/BP_InventoryComponent.BP_InventoryComponent_C") (Variables|InventoryData|GetItemID) (Variables|RepairDetails|GetRepairCost)))
    (bind _output_get (Variables|Default|SetIsCompleted _coulduseitem))
    (if _output_get
      (CallFunction|DisableInteraction)
      (Development|PrintString "Replaced")
      (Default|NotifyPieceCompleted (Variables|Default|GetOwnerRepairableItemReference) self)
      (CallFunction|SetRepairedMeshState true)
      (else
        (Development|PrintString "Not in Inventory or Not Enough Items")))))

(fn SetRepairedMeshState
  (params (ShowRepairedMesh :type Boolean))
  (Rendering|SetVisibility (Variables|Default|GetRepairedMesh) ShowRepairedMesh false)
  (Rendering|SetVisibility (Variables|Default|GetStaticMesh) (not ShowRepairedMesh) false))