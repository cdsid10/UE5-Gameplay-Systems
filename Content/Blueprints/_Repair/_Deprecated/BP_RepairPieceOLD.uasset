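; Deprecated repair piece actor that represents one fixable part of a larger repairable item.
; On interact, it compares the tool used with its required tool and prints a debug message on a mismatch.
; A match hides its mesh, turns off the box collision and notifies the owning repairable item that the piece is done.
; CanInteract always returns false, and the state getter and setter are empty stubs.
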(event Custom|Interact_1
  (params (Instigator :type BP%20Third%20Person%20Character%20Object%20Reference) (ToolToUse :type ERepairTool%20Enum :default "NewEnumerator0"))
  (CallFunction|TryRepair ToolToUse Instigator))

(event EventBeginPlay)

(event Collision|EventActorBeginOverlap
  (params (OtherActor :type Actor%20Object%20Reference)))

(event EventTick
  (params (DeltaSeconds :type Float%20%28single-precision%29)))

(fn ConstructionScript)

(fn CanInteract?
  (return false))

(fn TryRepair
  (params (ToolToUse :type ERepairTool%20Enum :default "NewEnumerator0") (Instigator :type BP%20Third%20Person%20Character%20Object%20Reference))
  (Variables|Default|SetPlayerCharacter Instigator)
  (if (Utilities|Enum|Equal(Enum) ToolToUse (Variables|RepairDetails|GetRequiredTool))
    (CallFunction|Repair)
    (else
      (Development|PrintString "Wrong Tool"))))

(fn EnableInteraction
  (Collision|SetCollisionEnabled (Variables|Default|GetBox_Collision) "QueryOnly"))

(fn DisableInteraction
  (Collision|SetCollisionEnabled (Variables|Default|GetBox_Collision) "NoCollision"))

(fn SetOwnerRepairableItemReference
  (params (OwnerRepairableItem :type BP%20Repairable%20Item%20Object%20Reference))
  (Variables|RepairDetails|SetOwnerRepairableItemReference OwnerRepairableItem))

(fn Repair
  (if true
    (Development|PrintString "Repaired")
    (Development|SetHiddeninGame (Variables|Default|GetStaticMesh) true false)
    (CallFunction|DisableInteraction)
    (Default|NotifyPieceCompleted (Variables|RepairDetails|GetOwnerRepairableItemReference) self)))

(fn GetState)

(fn SetState)