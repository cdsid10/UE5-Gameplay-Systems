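; Deprecated repairable item actor that runs a staged repair over its child BP_RepairPieceOLD actors.
; BeginPlay registers itself with each piece, and interaction toggles the interactor's repair menu and enters or exits repair mode on its BP_RepairComponent.
; StartRepair enables only pieces whose StepID matches the current stage.
; NotifyPieceCompleted advances the stage once those pieces are complete, or calls FinishRepair, which only prints a message.
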(event EventBeginPlay
  (Variables|RepairSequence|SetCurrentRepairStage 0)
  (for _array_element (Actor|GetAllChildActors true)
    (bind _asbp_repair_piece_old (Utilities|Casting|CastToBP_RepairPieceOLD _array_element))
    (Default|SetOwnerRepairableItemReference _asbp_repair_piece_old self)
    (Utilities|Array|AddUnique (Variables|Repair|GetRepairPieces) _asbp_repair_piece_old)))

(event Collision|EventActorBeginOverlap
  (params (OtherActor :type Actor%20Object%20Reference)))

(event EventTick
  (params (DeltaSeconds :type Float%20%28single-precision%29)))

(event EventInteract
  (params (Interactor :type BP%20Third%20Person%20Character%20Object%20Reference))
  (bind _returnvalue (Actor|GetComponentbyClass Interactor "/Game/Blueprints/_Repair/Player/BP_RepairComponent.BP_RepairComponent_C"))
  (Default|OpenCloseRepairMenu Interactor)
  (Utilities|IsValid _returnvalue
    (:Is%20Valid
      (Default|EnterRepairMode _returnvalue))))

(event EventEndInteraction
  (params (Interactor :type BP%20Third%20Person%20Character%20Object%20Reference))
  (bind _returnvalue (Actor|GetComponentbyClass Interactor "/Game/Blueprints/_Repair/Player/BP_RepairComponent.BP_RepairComponent_C"))
  (if (Variables|/Game/ThirdPerson/Blueprints/BP_ThirdPersonCharacter.BP_ThirdPersonCharacter_C|GetCanInteract Interactor)
    (Default|OpenCloseRepairMenu Interactor)
    (Utilities|IsValid _returnvalue
      (:Is%20Valid
        (Default|ExitRepairMode _returnvalue)))))

(fn ConstructionScript)

(fn StartRepair
  (for _array_element (Variables|Repair|GetRepairPieces)
    (LocalVariables|SetCurrentRepairPiece _array_element)
    (if (== (Variables|RepairSequence|GetCurrentRepairStage) (Variables|/Game/Blueprints/_Repair/_Deprecated/BP_RepairPieceOLD.BP_RepairPieceOLD_C|GetStepID (LocalVariables|GetCurrentRepairPiece)))
      (Default|EnableInteraction (LocalVariables|GetCurrentRepairPiece))
      (else
        (Default|DisableInteraction (LocalVariables|GetCurrentRepairPiece))))))

(fn NotifyPieceCompleted
  (params (CompletedRepairPiece :type BP%20Repair%20Piece%20OLD%20Object%20Reference))
  (LocalVariables|SetHasNextStage false)
  (Variables|RepairSequence|SetAllPiecesRepaired true)
  (bind _array_element (Utilities|Array|ForEachLoopwithBreak (Variables|Repair|GetRepairPieces) :!label _label)
    (:LoopBody
      (if (== (Variables|/Game/Blueprints/_Repair/_Deprecated/BP_RepairPieceOLD.BP_RepairPieceOLD_C|GetStepID _array_element) (Variables|RepairSequence|GetCurrentRepairStage))
        (if (not (Variables|/Game/Blueprints/_Repair/_Deprecated/BP_RepairPieceOLD.BP_RepairPieceOLD_C|GetIsCompleted _array_element))
          (Variables|RepairSequence|SetAllPiecesRepaired false)
          (goto _label Break))
        (elif (> (Variables|/Game/Blueprints/_Repair/_Deprecated/BP_RepairPieceOLD.BP_RepairPieceOLD_C|GetStepID _array_element) (Variables|RepairSequence|GetCurrentRepairStage))
          (LocalVariables|SetHasNextStage true))))
    (:Completed
      (if (Variables|RepairSequence|GetAllPiecesRepaired)
        (if (LocalVariables|GetHasNextStage)
          (CallFunction|ActivateNextRepairStage)
          (else
            (CallFunction|FinishRepair)))))))

(fn ActivateNextRepairStage
  (bind _currentrepairstage (Variables|RepairSequence|GetCurrentRepairStage))
  (Math|Integer|IncrementInt _currentrepairstage
    (:%20%20
      (Development|PrintString (Utilities|String|Append "Cuurent Repair Stage is: " (Utilities|String|ToString(Integer) _currentrepairstage)))
      (CallFunction|StartRepair))))

(fn FinishRepair
  (Development|PrintString "Repair is Finished!" true true "(R=1.000000,G=0.000000,B=0.089427,A=1.000000)"))